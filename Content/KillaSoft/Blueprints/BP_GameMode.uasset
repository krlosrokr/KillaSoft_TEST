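; Game mode Blueprint with empty event graphs and a single helper, AddWorldMarker, marked test-only, that attaches a floating icon marker to a given owner.
; AddWorldMarker adds a screen-space widget component above the owner and assigns it a newly constructed WB_Marker_World.
; It then sets the icon brush from the supplied material and tints it through the dynamic material's Color parameter.
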(event EventBeginPlay)

(event EventTick
  (params (DeltaSeconds :type Float%20%28single-precision%29)))

(fn ConstructionScript)

(fn AddWorldMarker
  (params (Owner :type Actor%20Object%20Reference) (Color :type Color%20Structure) (Material :type Material%20Interface%20Object%20Reference))
  ;[1 1 1] TEST ONLY
  (Utilities|FlowControl|Sequence
    (:then_0
      (bind _returnvalue (Game|AddComponentbyClass Owner "/Script/UMG.WidgetComponent" false))
      (bind _output_get (LocalVariables|SetWorldMarkerWidget _returnvalue))
      (bind _returnvalue_2 (Game|ConstructObjectfromClass "/Game/KillaSoft/Blueprints/HUD/Marker/WB_Marker_World.WB_Marker_World_C" "/Game/KillaSoft/Blueprints/HUD/Marker/WB_Marker_World.WB_Marker_World"))
      (bind _output_get_2 (LocalVariables|SetWorldMarker _returnvalue_2))
      (UserInterface|SetWidget _output_get _output_get_2)
      (Class|WidgetComponent|SetWidgetSpace _output_get "Screen")
      (Class|WidgetComponent|SetDrawSize _output_get "(X=50.000000,Y=50.000000)")
      (Transformation|SetRelativeLocation _output_get "0, 0,100.000000" false false))
    (:then_2
      (Class|Image|SetBrushfromMaterial (Variables|/Game/KillaSoft/Blueprints/HUD/Marker/WB_Marker_World.WB_Marker_World_C|GetMarkerIcon (LocalVariables|GetWorldMarker)) Material)
      (bind _returnvalue_3 (Appearance|GetDynamicMaterial (Variables|/Game/KillaSoft/Blueprints/HUD/Marker/WB_Marker_World.WB_Marker_World_C|GetMarkerIcon (LocalVariables|GetWorldMarker)) :!class /Script/UMG.Image))
      (Rendering|Material|SetVectorParameterValue _returnvalue_3 "Color" (Math|Conversions|ToLinearColor(Color) Color) :!class /Script/Engine.MaterialInstanceDynamic))))