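; BP_Marker is a HUD marker Blueprint that can test whether its owning actor is visible within the player's viewport.
; CheckIfOnScreen projects CurrentOwner's location to screen space for player 0 and requires a successful projection inside the viewport bounds, without any occlusion test.
; The event graph has no live logic, only unconnected test code that prints on-screen state, gated by ForcedHide, and distance from the actor.
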(event EventBeginPlay)

(event Collision|EventActorBeginOverlap
  (params (OtherActor :type Actor%20Object%20Reference)))

(event EventTick
  (params (DeltaSeconds :type Float%20%28single-precision%29)))

(fn ConstructionScript)

(fn CheckifonScreen
  (bind _returnvalue (Viewport|GetViewportSize))
  (bind _currentowner (Variables|Default|GetCurrentOwner)
    (:then
      (return (Math|Boolean|ANDBoolean (>= (.x (.ScreenPosition (Class|GameplayStatics|ProjectWorldtoScreen (Game|GetPlayerController 0) (Transformation|GetActorLocation _currentowner) false))) 0.0) (>= (.y (.ScreenPosition (Class|GameplayStatics|ProjectWorldtoScreen (Game|GetPlayerController 0) (Transformation|GetActorLocation _currentowner) false))) 0.0) (.ReturnValue (Class|GameplayStatics|ProjectWorldtoScreen (Game|GetPlayerController 0) (Transformation|GetActorLocation _currentowner) false)) (<= (.x (.ScreenPosition (Class|GameplayStatics|ProjectWorldtoScreen (Game|GetPlayerController 0) (Transformation|GetActorLocation _currentowner) false))) (.x _returnvalue)) (<= (.y (.ScreenPosition (Class|GameplayStatics|ProjectWorldtoScreen (Game|GetPlayerController 0) (Transformation|GetActorLocation _currentowner) false))) (.y _returnvalue)))))
    (:else)))