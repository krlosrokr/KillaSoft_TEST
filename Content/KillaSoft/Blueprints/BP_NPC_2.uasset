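; BP_NPC_2 is an NPC actor with a configurable color that registers a marker for itself through the game mode's MarkerManager.
; The construction script creates a dynamic material on the mesh and sets its BodyColor from NPCColor.
; On BeginPlay it creates a BP_Marker in that same color, then after a five-second delay prints a message and removes its reference from the manager.
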(event EventBeginPlay
  (CallFunction|SetMarkers)
  (Utilities|FlowControl|Delay 5.0)
  (CallFunction|ClearMarkers))

(event Collision|EventActorBeginOverlap
  (params (OtherActor :type Actor%20Object%20Reference)))

(event EventTick
  (params (DeltaSeconds :type Float%20%28single-precision%29)))

(fn ConstructionScript
  (CallFunction|SetColor))

(fn SetColor
  (bind _returnvalue (Rendering|Material|CreateDynamicMaterialInstance (Variables|Character|GetMesh) 0 0 "None" :!class /Script/Engine.PrimitiveComponent))
  (bind _output_get (Variables|Default|SetMat_Instance _returnvalue))
  (Rendering|Material|SetVectorParameterValue _output_get "BodyColor" (Math|Conversions|ToLinearColor(Color) (Variables|Default|GetNPC_Color)) :!class /Script/Engine.MaterialInstanceDynamic))

(fn SetMarkers
  ;[1 1 1] Add Marker
  (bind _asbp_game_mode (Utilities|Casting|CastToBP_GameMode (Game|GetGameMode)))
  (Class|KSTMarkerManagerComponent|CreateMarkerActor (Variables|/Game/KillaSoft/Blueprints/BP_GameMode.BP_GameMode_C|GetMarkerManager _asbp_game_mode) self "/Game/KillaSoft/Blueprints/HUD/Marker/BP_Marker.BP_Marker_C" (Variables|Default|GetNPC_Color) false))

(fn ClearMarkers
  (Utilities|FlowControl|Sequence
    (:then_0
      (Development|PrintString "Deleting this marker"))
    (:then_1
      (bind _asbp_game_mode (Utilities|Casting|CastToBP_GameMode (Game|GetGameMode)))
      (Class|KSTMarkerManagerComponent|RemoveActorRef (Variables|/Game/KillaSoft/Blueprints/BP_GameMode.BP_GameMode_C|GetMarkerManager _asbp_game_mode) self))))